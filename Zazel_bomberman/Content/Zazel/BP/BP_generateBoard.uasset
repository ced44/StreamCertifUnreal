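; Board generator actor that builds a grid centred on its root at BeginPlay, with an indestructible border.
; A coarse group grid, one entry per six interior cells per axis, gets a central group, a random non-central bumper and player groups elsewhere.
; A separate cell array, sized by NbY both ways, marks the border, spawned as BlocStatic instances.
; The group layout does not affect spawning; Tick prints it for debugging.
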(event EventBeginPlay
  (CallFunction|InitiateGroupBlock)
  (CallFunction|PopulateGroupBlock)
  (CallFunction|SetBoardStartGeneration)
  (CallFunction|PopulateCaseStructure)
  (CallFunction|InstanciateCaseStructure))

(event EventTick
  (params (DeltaSeconds :type Float%20%28single-precision%29))
  (CallFunction|DebugGroupCaseandPrint))

(fn ConstructionScript)

(fn SetBoardStartGeneration
  (Variables|Default|SetstartLocation (- (Transformation|GetWorldLocation (Variables|Default|GetDefaultSceneRoot)) (Math|Vector|MakeVector (/ (* (Variables|Default|GetnbX) (Variables|Default|GetcaseSizeUnit)) 2.0) (/ (* (Variables|Default|GetnbY) (Variables|Default|GetcaseSizeUnit)) 2.0) 0.0))))

(fn PopulateCaseStructure
  (bind _caseposition (Variables|Default|GetcasePosition))
  (Utilities|Array|Clear _caseposition)
  (Utilities|Array|Resize _caseposition (Variables|Default|GetnbY))
  (for (_ _array_index) _caseposition
    (CallFunction|AddEmptyArrayValue _array_index)
    (if (or (== _array_index 0) (== _array_index (Utilities|Array|LastIndex _caseposition)))
      (CallFunction|AddAllNonDestruct _array_index)
      (else
        (CallFunction|AddBeginandEndNnonDestruct _array_index)))))

(fn InstanciateCaseStructure
  (bind _casesizeunit (Variables|Default|GetcaseSizeUnit))
  (for (_array_element _array_index) (Variables|Default|GetcasePosition)
    (for (_array_element_2 _array_index_2) (.lineboard _array_element)
      (switch Utilities|FlowControl|Switch|Switchone_caseType _array_element_2
        (:NewEnumerator0
          (CallFunction|CreateNondestructCase (+ (Variables|Default|GetstartLocation) (Math|Vector|MakeVector (* _array_index _casesizeunit) (* _array_index_2 _casesizeunit) 0.0))))))))

(fn CreateNondestructCase
  (params (caseLocation :type Vector))
  (Components|InstancedStaticMesh|AddInstance (Variables|Default|GetblocStatic) (Math|Transform|MakeTransform caseLocation "0, 0, 0" "1,1,1")))

(fn AddAllNonDestruct
  (params (nbLine :type Integer))
  (bind _caseposition (Variables|Default|GetcasePosition))
  (bind _output (Utilities|Array|Get(acopy) _caseposition nbLine))
  (for (_ _array_index) (.lineboard _output)
    (Utilities|Array|SetArrayElem (.lineboard _output) _array_index "NewEnumerator0")))

(fn AddBeginandEndNnonDestruct
  (params (indexArrayLine :type Integer))
  (bind _caseposition (Variables|Default|GetcasePosition))
  (bind _output (Utilities|Array|Get(acopy) _caseposition indexArrayLine))
  (Utilities|Array|SetArrayElem (.lineboard _output) 0 "NewEnumerator0")
  (Utilities|Array|SetArrayElem (.lineboard _output) (Utilities|Array|LastIndex (.lineboard _output)) "NewEnumerator0"))

(fn AddEmptyArrayValue
  (params (index :type Integer))
  (for _index (range 1 (Variables|Default|GetnbY))
    (Utilities|Array|Add (.lineboard (Utilities|Array|Get(acopy) (Variables|Default|GetcasePosition) index)) "NewEnumerator4")))

(fn InitiateGroupBlock
  (bind _groupcaseposition (Variables|Default|GetgroupCasePosition))
  (Utilities|Array|Clear _groupcaseposition)
  (Utilities|Array|Resize _groupcaseposition (/ (- (Variables|Default|GetnbY) 2) 6))
  (for (_ _array_index) (Variables|Default|GetgroupCasePosition)
    (for _index (range 1 (/ (- (Variables|Default|GetnbX) 2) 6))
      (Utilities|Array|Add (.gouplineboard (Utilities|Array|Get(acopy) (Variables|Default|GetgroupCasePosition) _array_index)) "NewEnumerator0"))))

(fn PopulateGroupBlock
  (CallFunction|SetGroupCentral)
  (CallFunction|SetGroupBumper)
  (CallFunction|SetGroupsPlayer))

(fn SetGroupCentral
  (bind _groupcaseposition (Variables|Default|GetgroupCasePosition))
  (bind _groupcaseposition_2 (Variables|Default|GetgroupCasePosition))
  (bind _returnvalue (Utilities|Array|Length _groupcaseposition))
  (bind _returnvalue_2 (Utilities|MGetCentralIndex _returnvalue))
  (bind _output (Utilities|Array|Get(acopy) _groupcaseposition_2 _returnvalue_2))
  (bind _returnvalue_3 (Utilities|Array|Length (.gouplineboard _output)))
  (bind _returnvalue_4 (Utilities|MGetCentralIndex _returnvalue_3))
  (Variables|Default|SetcoordYCentral _returnvalue_2)
  (Variables|Default|SetcoordXCentral _returnvalue_4)
  (Utilities|Array|SetArrayElem (.gouplineboard _output) _returnvalue_4 "NewEnumerator2"))

(fn DebugGroupCaseandPrint
  (bind _arrayelement (Utilities|Array|ReverseforEachLoop (Variables|Default|GetgroupCasePosition))
    (:LoopBody
      (bind _output_get (LocalVariables|SetdebugString ""))
      (for _array_element (.gouplineboard _arrayelement)
        (bind _output_get_2 (LocalVariables|SetdebugString (Utilities|String|Append _output_get "   " (Utilities|String|EnumtoString _array_element)))))
      (Development|PrintString _output_get_2 true true "(R=0.000000,G=0.660000,B=1.000000,A=1.000000)" 0.0))))

(fn SetGroupBumper
  (Variables|Default|SetnbGroupCaseY (Utilities|Array|Length (Variables|Default|GetgroupCasePosition)))
  (Development|PrintString (Utilities|String|ToString(Text) (Utilities|Text|FormatText "nbGroupCaseY = {nbGroupCaseY}" (Variables|Default|GetnbGroupCaseY))) true true "(R=0.000000,G=0.660000,B=1.000000,A=1.000000)" 5.0)
  (Variables|Default|SetnbGroupCaseX (Utilities|Array|Length (.gouplineboard (Utilities|Array|Get(acopy) (Variables|Default|GetgroupCasePosition)))))
  (Development|PrintString (Utilities|String|ToString(Text) (Utilities|Text|FormatText "nbGroupCaseX = {nbGroupCaseX}" (Variables|Default|GetnbGroupCaseX))) true true "(R=0.000000,G=0.660000,B=1.000000,A=1.000000)" 5.0)
  (CallFunction|RandomBumperCoord :!label _label)
  (if (and (== (Variables|Default|GetcoordYBumper) (Variables|Default|GetcoordYCentral)) (== (Variables|Default|GetcoordXBumper) (Variables|Default|GetcoordXCentral)))
    (goto _label)
    (else
      (Utilities|Array|SetArrayElem (.gouplineboard (Utilities|Array|Get(acopy) (Variables|Default|GetgroupCasePosition) (Variables|Default|GetcoordYBumper))) (Variables|Default|GetcoordXBumper) "NewEnumerator3")
      (Development|PrintString (Utilities|String|ToString(Text) (Utilities|Text|FormatText "nb colonne post traitement = {x}" (Utilities|Array|Length (.gouplineboard (Utilities|Array|Get(acopy) (Variables|Default|GetgroupCasePosition) (Variables|Default|GetcoordYBumper)))))) true true "(R=0.000000,G=0.660000,B=1.000000,A=1.000000)" 1e+02))))

(fn RandomBumperCoord
  (Variables|Default|SetcoordYBumper (Math|Random|RandomInteger (Variables|Default|GetnbGroupCaseY)))
  (Development|PrintString (Utilities|String|ToString(Text) (Utilities|Text|FormatText "coordY Bumper = {coordYBumper}" (Variables|Default|GetcoordYBumper))) true true "(R=0.000000,G=0.660000,B=1.000000,A=1.000000)" 1e+02)
  (Variables|Default|SetcoordXBumper (Math|Random|RandomInteger (Variables|Default|GetnbGroupCaseX)))
  (Development|PrintString (Utilities|String|ToString(Text) (Utilities|Text|FormatText "coordX Bumper = {coordXBumper}" (Variables|Default|GetcoordXBumper))) true true "(R=0.000000,G=0.660000,B=1.000000,A=1.000000)" 1e+02))

(fn SetGroupsPlayer
  (for (_array_element _array_index) (Variables|Default|GetgroupCasePosition)
    (for (_array_element_2 _array_index_2) (.gouplineboard _array_element)
      (switch Utilities|FlowControl|Switch|Switchone_groupeCaseType _array_element_2
        (:NewEnumerator0
          (Utilities|Array|SetArrayElem (.gouplineboard (Utilities|Array|Get(acopy) (Variables|Default|GetgroupCasePosition) _array_index)) _array_index_2 "NewEnumerator1"))))))