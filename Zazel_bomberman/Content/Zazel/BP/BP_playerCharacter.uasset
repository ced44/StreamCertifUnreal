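; Player character for a bomb-placing game, handling movement input, bomb drops and a bomb-hit event that only prints a death message.
; The bomb input passes through a DoOnce that resets after a short delay as a cooldown.
; Bombs spawn at a grid-snapped point ahead of the capsule, unless a debug-drawn, effectively zero-length sphere trace detects something already there.
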(event Custom|fn_bombInstanciated
  (Utilities|FlowControl|DoOnce false
    (:Completed
      ;[1 1 1] use to instanciate Bomb
      (CallFunction|FnInstanciateBomb)
      (Utilities|FlowControl|Delay 0.2)
      (CallFunction|EvtCooldownBomb))))

(event Custom|evt_cooldownBomb
  (Utilities|FlowControl|DoOnce false) ; enters at Reset
)

(event EventFnDamageBomb
  (Development|PrintString "You died !" true true "(R=1.000000,G=0.199368,B=0.000000,A=1.000000)" 5.0))

(event Input|ActionEvents|InputActioninput_putBomb
  (params (Key :type Key%20Structure :default "None"))
  (:Pressed
    (CallFunction|FnBombInstanciated)))

(event Input|AxisEvents|InputAxisinput_TopDown
  (params (AxisValue :type Float%20%28single-precision%29))
  ;[1 1 1] topDownDp
  (Pawn|Input|AddMovementInput (Math|Vector|MakeVector AxisValue (Input|AxisValues|Getinput_LeftRight) 0.0) 1.0 false))

(fn ConstructionScript)

(fn FnInstanciateBomb
  (bind _capsulecomponent (Variables|Collision|GetCapsuleComponent))
  (bind _output_get (LocalVariables|SetbombPosition (Class|KismetMathLibrary|VectorSnappedtoGrid (+ (Transformation|GetWorldLocation _capsulecomponent) (* (Math|Vector|GetForwardVector _capsulecomponent) 100)) 1e+02)))
  (bind _returnvalue (Collision|SphereTraceByChannel (+ _output_get "0, 0,1.000000") (- _output_get "0, 0,-1.000000") 5e+01 "TraceTypeQuery1" false 0 "ForDuration"))
  (if _returnvalue
    (Development|PrintString "collide" true true "(R=1.000000,G=0.133002,B=0.000000,A=1.000000)")
    (else
      (Game|SpawnActorfromClass "/Game/Zazel/BP/BP_Bomb.BP_Bomb_C" (Math|Transform|MakeTransform (LocalVariables|GetbombPosition) "0, 0, 0" "1,1,1") "AdjustIfPossibleButAlwaysSpawn" 0 3 0))))