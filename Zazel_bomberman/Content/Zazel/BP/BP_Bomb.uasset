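; Bomberman-style bomb actor that, after a short fuse from BeginPlay, blasts in a cross shape and destroys itself after a further delay.
; MultiTrace fires TraceBomb along ±X and ±Y, with reach set by NbCase in 100-unit cells.
; Each single sphere trace on Visibility sends the BPI_Damage bomb message to its first hit if implemented, otherwise prints a debug string; traces are debug-drawn.
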(event EventBeginPlay
  (Utilities|FlowControl|Delay 3.0)
  (CallFunction|MultiTrace (Variables|Default|GetNb%20Case))
  (Utilities|FlowControl|Delay 2.0)
  (Actor|DestroyActor))

(fn ConstructionScript)

(fn TraceBomb
  (params (End :type Vector))
  (bind _bomb (Variables|Default|Getbomb))
  (bind _returnvalue (Transformation|GetWorldLocation _bomb))
  (bind (_outhit _returnvalue_2) (Collision|SphereTraceByChannel _returnvalue (+ _returnvalue End) 45.0 "TraceTypeQuery1" false 0 "ForDuration"))
  (if (and (Utilities|DoesObjectImplementInterface (.HitActor (Collision|BreakHitResult _outhit)) "/Game/Zazel/BP/BPI_Damage.BPI_Damage_C") _returnvalue_2)
    (Class|BPIDamage|FnDamageBomb(Message) (.HitActor (Collision|BreakHitResult _outhit)))
    (else
      (Development|PrintString "Coliide"))))

(fn MultiTrace
  (params (nbCase :type Integer))
  (bind _returnvalue (* nbCase 1e+02))
  (bind _returnvalue_2 (* -1.0 _returnvalue))
  (CallFunction|TraceBomb (Math|Vector|MakeVector _returnvalue 0.0 0.0))
  (CallFunction|TraceBomb (Math|Vector|MakeVector _returnvalue_2 0.0 0.0))
  (CallFunction|TraceBomb (Math|Vector|MakeVector 0.0 _returnvalue 0.0))
  (CallFunction|TraceBomb (Math|Vector|MakeVector 0.0 _returnvalue_2 0.0)))